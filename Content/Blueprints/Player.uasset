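; Player pawn with axis-driven movement and a jump gated by a Grounded flag.
; The forward/back and left/right axes feed AddMovementInput along the actor's forward and right vectors.
; Jump applies an upward JumpForce to the StaticMesh through AddForce and clears Grounded.
; The Hit event sets Grounded again whenever the hit normal is not exactly straight up, so walls and other non-flat contacts also re-enable jumping.
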(event `self.ReceiveHit`
  (params (MyComp :type "PrimitiveComponent Object Reference") (Other :type "Actor Object Reference") (OtherComp :type "PrimitiveComponent Object Reference") (bSelfMoved :type Boolean) (HitLocation :type "Vector Structure") (HitNormal :type "Vector Structure") (NormalImpulse :type "Vector Structure") (Hit :type "HitResult Structure (by ref)"))
  ;[1 1 1] Grounded?
  (if (`KismetMathLibrary.NotEqualExactly_VectorVector` HitNormal (0.0 0.0 1.0))
    (set `self.Grounded` true)))

(event `InputAxis|Move_ForwardBack`
  (params (AxisValue :type "Float (single-precision)"))
  ;[1 1 1] Movement
  (`self.AddMovementInput` (`self.GetActorForwardVector`) AxisValue))

(event `InputAxis|Move_LeftRight`
  (params (AxisValue :type "Float (single-precision)"))
  ;[1 1 1] Movement
  (`self.AddMovementInput` (`self.GetActorRightVector`) AxisValue))

(event `InputAction|Jump`
  (params (Key :type "Key Structure"))
  ;[1 1 1] Jumping
  (:`Pressed`
    (if (`self.Grounded`)
      (`PrimitiveComponent.AddForce` (`self.StaticMesh`) (* (`KismetMathLibrary.Vector_Up`) (`self.JumpForce`)) "None" false)
      (set `self.Grounded` false))))

(fn `UserConstructionScript`)